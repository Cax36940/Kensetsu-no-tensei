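; BP_bullet is a turret projectile that damages what it hits according to its damage type.
; On BeginPlay it applies any supplied mesh and material to its Sphere, and enables homing toward its target only when the material is valid.
; On hit it switches on DamageType, handing poison, flat, area blast or magic damage to the BPCAttacks component.
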(event EventBeginPlay
  ;[1 1 1] set mesh
  (bind _bulletmesh (Variables|Default|GetBulletMesh)
    (:then
      (Components|StaticMesh|SetStaticMesh (Variables|Default|GetSphere) _bulletmesh))
    (:else
      _))
  (bind _bulletmaterial (Variables|Default|GetBulletMaterial)
    (:then
      (Rendering|Material|SetMaterial (Variables|Default|GetSphere) 0 _bulletmaterial)
      (Variables|/Script/Engine.ProjectileMovementComponent|SetHomingTargetComponent (Variables|Default|GetProjectileMovement) (Variables|Default|GetHoming%20Target%20Component))
      (Variables|/Script/Engine.ProjectileMovementComponent|SetbIsHomingProjectile (Variables|Default|GetProjectileMovement) true))
    (:else)))

(event Collision|EventHit
  (params (MyComp :type Primitive%20Component%20Object%20Reference) (Other :type Actor%20Object%20Reference) (OtherComp :type Primitive%20Component%20Object%20Reference) (bSelfMoved :type Boolean) (HitLocation :type Vector :default "0, 0, 0") (HitNormal :type Vector :default "0, 0, 0") (NormalImpulse :type Vector :default "0, 0, 0") (Hit :type Hit%20Result%20Structure%20%28by%20ref%29))
  ;[1 1 1] Damage enemy
  (switch Utilities|FlowControl|Switch|SwitchonDamage_Type (Variables|Default|GetDamageType)
    (:NewEnumerator0
      (Default|Poison (Variables|Default|GetBPC_Attacks) Other (Variables|Default|GetDamage) 3.0 0.5))
    (:NewEnumerator1
      (Default|Flat (Variables|Default|GetBPC_Attacks) Other (Variables|Default|GetDamage)))
    (:NewEnumerator2
      (Default|Blast (Variables|Default|GetBPC_Attacks) (Variables|Default|GetDamage) 2e+02))
    (:NewEnumerator3
      (Default|Magic (Variables|Default|GetBPC_Attacks) Other (Variables|Default|GetDamage) 4e+02 3.0))))

(fn ConstructionScript)