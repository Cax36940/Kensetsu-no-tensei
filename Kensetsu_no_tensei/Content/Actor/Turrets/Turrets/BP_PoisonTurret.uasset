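; Poison turret Blueprint that adds an idle spin-and-bob animation to its Top component, with no poison or attack logic of its own.
; BeginPlay calls the parent and caches the Top's relative location as the base position.
; Tick rotates the Top by a fixed step per frame, independent of delta time, and offsets its height with a sine of accumulated time.
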(event Collision|EventActorBeginOverlap
  (params (OtherActor :type Actor%20Object%20Reference))
  (|CallParentFunction OtherActor) ; This node is disabled and will not be called.\nDrag off pins to build functionality.
)

(event EventTick
  (params (DeltaSeconds :type Float%20%28single-precision%29))
  (|CallParentFunction DeltaSeconds)
  (Transformation|AddLocalRotation (Variables|Default|GetTop) "0.000000,0.500000,0.000000" false false)
  (bind _output_get (Variables|Default|SetTopPositionTimer (+ (Variables|Default|GetTopPositionTimer) DeltaSeconds)))
  (Transformation|SetRelativeLocation (Variables|Default|GetTop) (+ (Variables|Default|GetTopPosition) (Math|Vector|MakeVector 0.0 0.0 (* (Math|Trig|Sin(Radians) _output_get) 1e+01))) false false))

(event EventBeginPlay
  (|CallParentFunction)
  (Variables|Default|SetTopPosition (Variables|/Script/Engine.SceneComponent|GetRelativeLocation (Variables|Default|GetTop)))
  (Variables|Default|SetTopPositionTimer 0.0))

(fn ConstructionScript
  (|CallParentFunction))