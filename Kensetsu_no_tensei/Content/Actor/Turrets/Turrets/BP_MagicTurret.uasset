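; BP_MagicTurret is a turret Blueprint that animates its Top component, with no targeting or firing logic of its own.
; BeginPlay caches Top's relative location, and Tick applies a fixed rotation step each frame, so spin speed depends on frame rate.
; A sine-based vertical bob is unfinished: its time variable resets to zero, the increment is unused and Sin receives zero, so Top stays at its cached height.
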(event EventBeginPlay
  (|CallParentFunction)
  (Variables|Default|SetTopPosition (Variables|/Script/Engine.SceneComponent|GetRelativeLocation (Variables|Default|GetTop)))
  (Variables|Default|SetTopPositionTIme 0.0))

(event Collision|EventActorBeginOverlap
  (params (OtherActor :type Actor%20Object%20Reference))
  (|CallParentFunction OtherActor) ; This node is disabled and will not be called.\nDrag off pins to build functionality.
)

(event EventTick
  (params (DeltaSeconds :type Float%20%28single-precision%29))
  (|CallParentFunction DeltaSeconds)
  (Transformation|AddLocalRotation (Variables|Default|GetTop) "0.000000,0.500000,0.000000" false false)
  (Variables|Default|SetTopPositionTIme 0.0)
  (Transformation|SetRelativeLocation (Variables|Default|GetTop) (+ (Variables|Default|GetTopPosition) (Math|Vector|MakeVector 0.0 0.0 (* (Math|Trig|Sin(Radians) 0.0) 1e+01))) false false))

(fn ConstructionScript
  (|CallParentFunction))