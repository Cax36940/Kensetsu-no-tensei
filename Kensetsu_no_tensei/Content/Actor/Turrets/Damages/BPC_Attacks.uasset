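; Actor component for the turret damage system that provides the Flat, Poison, Blast and Magic attack types as events.
; Flat applies damage and destroys the owning actor, and Magic simply forwards to it.
; Poison spawns a Poison_Damage actor configured for damage over time on the target.
; Blast spawns an AOE_Blast at the owner's location and binds its overlap event to route each reported actor through Flat, which also destroys the owner.
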(event Custom|Poison
  (params (DamagedActor :type Actor%20Object%20Reference) (DamageOnTick :type Float%20%28single-precision%29) (Duration :type Float%20%28double-precision%29) (SpawnInterval :type Float%20%28double-precision%29))
  (Game|SpawnActorfromClass "/Game/Actor/Turrets/Damages/Poison_Damage.Poison_Damage_C" (Math|Transform|MakeTransform "0, 0, 0" "0, 0, 0" "1.000000,1.000000,1.000000") "Undefined" "MultiplyWithRoot" 0 DamagedActor DamageOnTick Duration SpawnInterval 0))

(event Custom|Flat
  (params (Target :type Actor%20Object%20Reference) (BaseDamage :type Float%20%28single-precision%29))
  (Game|Damage|ApplyDamage Target BaseDamage 0 0)
  (Actor|DestroyActor (Components|GetOwner)))

(event Custom|Blast
  (params (BaseDamage :type Float%20%28single-precision%29))
  (bind _returnvalue (Game|SpawnActorfromClass "/Game/Actor/Turrets/Damages/AOE_Blast.AOE_Blast_C" (Math|Transform|MakeTransform (Transformation|GetActorLocation (Components|GetOwner)) "0, 0, 0" "1.000000,1.000000,1.000000") "Undefined" "MultiplyWithRoot" 0 0))
  (EventDispatchers|BindEventtoOnAOEOverlapActor _returnvalue (delegate Custom|DamageEnemyAOE))
  (Default|SpawnSphere _returnvalue))

(event Custom|DamageEnemyAOE
  (params (Actor :type Actor%20Object%20Reference))
  (Development|PrintString (Utilities|GetDisplayName Actor))
  (CallFunction|Flat Actor (stale Custom|Blast BaseDamage)))

(event Custom|Magic
  (params (Target :type Actor%20Object%20Reference) (BaseDamage :type Float%20%28single-precision%29))
  (CallFunction|Flat Target BaseDamage))

(event EventBeginPlay)

(event EventTick
  (params (DeltaSeconds :type Float%20%28single-precision%29)))

(fn BPCAttacksAutoGenFunc
  (params (NewParam :type Float%20%28double-precision%29) (NewParam1 :type Float%20%28double-precision%29)))