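; Manages tower-defense turret placement and removal on BP_Grid, using a spawned BP_Turret as a grid-snapped cursor preview.
; Each tick, BuildMode moves, shows or hides the preview, whose meshes, material and range ring follow the tile underneath.
; Placing spawns that tile's turret class and charges UI_PlayerInterface if affordable.
; Removing destroys the turret nearest the cursor and refunds 90% of its total cost.
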(event Custom|PlaceTurret
  (bind _cursorturret (Variables|Default|GetCursorTurret))
  (bind _returnvalue (Transformation|GetActorLocation _cursorturret))
  ;[1 1 1] Place Turret
  (bind _hasenough (Default|CanPay (Variables|Default|GetUI_playerInterface) (Variables|Default|GetCostTurret)))
  (if _hasenough
    (if (!= (.z _returnvalue) -1e+03)
      (bind _gridposition (Default|GetNearestGridCell (Variables|Default|GetGrid) (Math|Vector|MakeVector (.x _returnvalue) (.y _returnvalue) 0.0)))
      (bind _result (Default|GridPositionIsinGrid (Variables|Default|GetGrid) _gridposition))
      (if _result
        (bind _isadded (Default|PlaceTower (Variables|Default|GetGrid) _gridposition))
        (if _isadded
          (CallFunction|CreateTurret)
          (Default|Pay (Variables|Default|GetUI_playerInterface) (Variables|Default|GetCostTurret)))))))

(event Custom|RemoveTurret
  (bind _cursorturret (Variables|Default|GetCursorTurret))
  (bind _returnvalue (Transformation|GetActorLocation _cursorturret))
  ;[1 1 1] RemoveTurret
  (bind _gridposition (Default|GetNearestGridCell (Variables|Default|GetGrid) (Math|Vector|MakeVector (.x _returnvalue) (.y _returnvalue) 0.0)))
  (bind _towerwasremoved (Default|RemoveTower (Variables|Default|GetGrid) _gridposition))
  (if _towerwasremoved
    (bind _target (CallFunction|TurrettobeDestroyed (Transformation|GetActorLocation (Variables|Default|GetCursorTurret))))
    (Default|GainMoney (Variables|Default|GetUI_playerInterface) (Math|Float|Truncate (* (Math|Conversions|ToFloat(Integer) (Variables|/Game/Actor/Turrets/BP_Turret.BP_Turret_C|GetCostTotal _target)) 0.9)))
    (Actor|DestroyActor _target)))

(event EventBeginPlay
  ;[1 1 1] Initialise Cursor Turret
  (bind _returnvalue (Game|SpawnActorfromClass "/Game/Actor/Turrets/BP_Turret.BP_Turret_C" (Math|Transform|MakeTransform "0.000000,0.000000,-1000.000000" "0, 0, 0" "1.000000,1.000000,1.000000") "Undefined" "MultiplyWithRoot" 0 0 0 0 0 0.0 0))
  (Variables|Default|SetCursorTurret _returnvalue)
  ;[1 1 1] init grid
  (bind _returnvalue_2 (Actor|GetActorOfClass "/Game/Blueprint/BP_Grid.BP_Grid_C"))
  (Variables|Default|SetGrid _returnvalue_2)
  (Utilities|FlowControl|Delay 0.2)
  ;[1 1 1] init player interface (for money)
  (bind _foundwidgets (Widget|GetAllWidgetsOfClass "/Game/UI/UI_PlayerInterface.UI_PlayerInterface_C" true))
  (Variables|Default|SetUI_playerInterface (Utilities|Array|Get(acopy) _foundwidgets)))

(event EventTick
  (params (DeltaSeconds :type Float%20%28single-precision%29))
  (Utilities|FlowControl|Sequence
    (:then_0
      (if (== (Variables|Default|GetBuildMode) "Tower")
        (CallFunction|MoveCursorBuildTuret)
        (CallFunction|BuildTurretHide/show)))
    (:then_1
      (if (== (Variables|Default|GetBuildMode) "Destroy")
        (CallFunction|MoveCursorDestroyTurret)
        (CallFunction|DestroyTurretHide/show)))
    (:then_2
      (if (== (Variables|Default|GetBuildMode) "")
        (Transformation|SetActorLocation (Variables|Default|GetCursorTurret) "0.000000,0.000000,-1000.000000" false false)
        (Rendering|SetActorHiddenInGame (Variables|Default|GetCursorTurret) true)))))

(fn ConstructionScript)

(fn MoveCursorBuildTuret
  (bind _returnvalue (Game|GetPlayerController 0))
  (bind _hitresult (Game|Player|GetHitResultUnderCursorbyChannel _returnvalue "TraceTypeQuery1" true))
  (bind _returnvalue_2 (+ (.y (.impactpoint _hitresult)) 1e+02))
  (bind _returnvalue_3 (+ (.x (.impactpoint _hitresult)) 1e+02))
  (bind _returnvalue_4 (Math|Float|%(Float) _returnvalue_2 2e+02))
  (bind _returnvalue_5 (Math|Float|%(Float) _returnvalue_3 2e+02))
  (bind _returnvalue_6 (- _returnvalue_2 _returnvalue_4))
  (bind _returnvalue_7 (- _returnvalue_3 _returnvalue_5))
  (bind _returnvalue_8 (Math|Vector|MakeVector _returnvalue_7 _returnvalue_6 1e+02))
  ;[1 1 1] Move Cursor
  (Transformation|SetActorLocation (Variables|Default|GetCursorTurret) _returnvalue_8 false false)
  ;[1 1 1] Change Mesh
  (bind _gridposition (Default|GetNearestGridCell (Variables|Default|GetGrid) _returnvalue_8))
  (bind _result (Default|GridPositionIsinGrid (Variables|Default|GetGrid) _gridposition))
  (if _result
    (bind _terraintile (Default|GetTileatPos (Variables|Default|GetGrid) _gridposition))
    (CallFunction|ChangeCursorMesh _terraintile (Variables|/Game/Actor/Terrains/BP_TerrainTile.BP_TerrainTile_C|GetTurretMaterial _terraintile) (Variables|/Game/Actor/Terrains/BP_TerrainTile.BP_TerrainTile_C|GetTurretRange _terraintile))))

(fn CreateTurret
  (Game|SpawnActorfromClass (Variables|Default|GetTurret%20Class) (Transformation|GetActorTransform (Variables|Default|GetCursorTurret)) "Undefined" "MultiplyWithRoot" 0 0 0 0 0 0.0 0)
  (return))

(fn MoveCursorDestroyTurret
  (bind _returnvalue (Game|GetPlayerController 0))
  (bind _hitresult (Game|Player|GetHitResultUnderCursorbyChannel _returnvalue "TraceTypeQuery1" true))
  (bind _returnvalue_2 (+ (.y (.impactpoint _hitresult)) 1e+02))
  (bind _returnvalue_3 (+ (.x (.impactpoint _hitresult)) 1e+02))
  (bind _returnvalue_4 (Math|Float|%(Float) _returnvalue_3 2e+02))
  (bind _returnvalue_5 (Math|Float|%(Float) _returnvalue_2 2e+02))
  (bind _returnvalue_6 (- _returnvalue_2 _returnvalue_5))
  (bind _returnvalue_7 (- _returnvalue_3 _returnvalue_4))
  (bind _returnvalue_8 (Math|Vector|MakeVector _returnvalue_7 _returnvalue_6 1e+02))
  ;[1 1 1] Move Cursor
  (Transformation|SetActorLocation (Variables|Default|GetCursorTurret) _returnvalue_8 false false)
  ;[1 1 1] Change Mesh
  (bind _gridposition (Default|GetNearestGridCell (Variables|Default|GetGrid) _returnvalue_8))
  (bind _result (Default|GridPositionIsinGrid (Variables|Default|GetGrid) _gridposition))
  (if _result
    (bind _terraintile (Default|GetTileatPos (Variables|Default|GetGrid) _gridposition))
    (CallFunction|ChangeCursorMesh _terraintile "/Game/Mesh/Towers/Archer/TowerDeleteMaterial.TowerDeleteMaterial" 0.0)))

(fn TurrettobeDestroyed
  (params (Position :type Vector))
  (bind _outactors (Actor|GetAllActorsOfClass "/Game/Actor/Turrets/BP_Turret.BP_Turret_C"))
  (if (!= (Utilities|Array|Get(acopy) _outactors) (Variables|Default|GetCursorTurret))
    (LocalVariables|SetNearest (Utilities|Array|Get(acopy) _outactors))
    (else
      (LocalVariables|SetNearest (Utilities|Array|Get(acopy) _outactors 1))))
  (for _array_element _outactors
    (if (and (!= (Variables|Default|GetCursorTurret) _array_element) (< (Math|Vector|Distance(Vector) (Transformation|GetActorLocation _array_element) Position) (Math|Vector|Distance(Vector) (Transformation|GetActorLocation (LocalVariables|GetNearest)) Position)))
      (LocalVariables|SetNearest _array_element)))
  (return (LocalVariables|GetNearest)))

(fn BuildTurretHide/show
  (bind _grid (Variables|Default|GetGrid))
  (bind _cursorturret (Variables|Default|GetCursorTurret))
  (bind _returnvalue (Transformation|GetActorLocation _cursorturret))
  (bind _gridposition (Default|GetNearestGridCell _grid (Math|Vector|MakeVector (.x _returnvalue) (.y _returnvalue) 0.0)))
  (bind _result (Default|GridPositionIsinGrid _grid _gridposition))
  (if _result
    (bind _isgridtilefree (Default|IsTileFree _grid _gridposition))
    (Rendering|SetActorHiddenInGame (Variables|Default|GetCursorTurret) (not _isgridtilefree))
    (Transformation|SetActorScale3D (Variables|Default|GetCursorTurret) "1.000000,1.000000,1.000000")
    (else
      (Rendering|SetActorHiddenInGame (Variables|Default|GetCursorTurret) true))))

(fn DestroyTurretHide/show
  (bind _grid (Variables|Default|GetGrid))
  (bind _cursorturret (Variables|Default|GetCursorTurret))
  (bind _returnvalue (Transformation|GetActorLocation _cursorturret))
  (bind _gridposition (Default|GetNearestGridCell _grid (Math|Vector|MakeVector (.x _returnvalue) (.y _returnvalue) 0.0)))
  (bind _result (Default|GridPositionIsinGrid _grid _gridposition))
  (if _result
    (bind _isroadtile (Default|IsTileRoad _grid _gridposition))
    (bind _istiletower (Default|IsTileTower _grid _gridposition))
    (Rendering|SetActorHiddenInGame (Variables|Default|GetCursorTurret) (not (and (not _isroadtile) _istiletower)))
    (Transformation|SetActorScale3D (Variables|Default|GetCursorTurret) "1.100000,1.100000,1.100000")
    (else
      (Rendering|SetActorHiddenInGame (Variables|Default|GetCursorTurret) true))))

(fn ChangeCursorMesh
  (params (TerrainTile :type BP%20Terrain%20Tile%20Object%20Reference) (Material :type Material%20Instance%20Object%20Reference) (Range :type Float%20%28double-precision%29))
  (bind _cursorturret (Variables|Default|GetCursorTurret))
  (bind _cursorturret_2 (Variables|Default|GetCursorTurret))
  (bind _cursorturret_3 (Variables|Default|GetCursorTurret))
  (bind _returnvalue (Actor|GetComponentsByClass _cursorturret "/Script/Engine.StaticMeshComponent"))
  (bind _returnvalue_2 (Actor|GetComponentsByClass _cursorturret_2 "/Script/Engine.StaticMeshComponent"))
  (bind _returnvalue_3 (Actor|GetComponentsByClass _cursorturret_3 "/Script/Engine.StaticMeshComponent"))
  (bind _returnvalue_4 (/ Range 5e+01))
  (bind _output (Utilities|Array|Get(acopy) _returnvalue 1))
  (bind _output_2 (Utilities|Array|Get(acopy) _returnvalue_3 2))
  (bind _output_3 (Utilities|Array|Get(acopy) _returnvalue_2))
  (Variables|Default|SetTurret%20Class (Variables|/Game/Actor/Terrains/BP_TerrainTile.BP_TerrainTile_C|GetTurretClass TerrainTile))
  ;[1 1 1] Set Base Mesh
  (Components|StaticMesh|SetStaticMesh _output_3 (Variables|/Game/Actor/Terrains/BP_TerrainTile.BP_TerrainTile_C|GetTurretBaseMesh TerrainTile))
  (Rendering|Material|SetMaterial _output_3 0 Material)
  ;[1 1 1] Set Top Mesh
  (Components|StaticMesh|SetStaticMesh _output (Variables|/Game/Actor/Terrains/BP_TerrainTile.BP_TerrainTile_C|GetTurretTopMesh TerrainTile))
  (Rendering|Material|SetMaterial _output 0 Material)
  ;[1 1 1] Set Range
  (Rendering|SetVisibility _output_2 true false)
  (Transformation|SetRelativeScale3D _output_2 (Math|Vector|MakeVector _returnvalue_4 _returnvalue_4 1.0)))