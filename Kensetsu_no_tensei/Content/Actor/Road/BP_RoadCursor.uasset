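; BP_RoadCursor is a cursor actor that indicates whether a road can be placed or deleted.
; ShowRoad and ShowCross each call HideAll, then reveal the Road or Cross component and set the matching CanPlaceRoad or CanDeleteRoad flag.
; HideAll hides mesh components among the root's direct children and clears both flags.
; The event graph is empty, so the cursor changes state only when these functions are called.
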(event EventBeginPlay)

(event Collision|EventActorBeginOverlap
  (params (OtherActor :type Actor%20Object%20Reference)))

(event EventTick
  (params (DeltaSeconds :type Float%20%28single-precision%29)))

(fn ConstructionScript)

(fn ShowRoad
  (CallFunction|HideAll)
  (Rendering|SetVisibility (Variables|Default|GetRoad) true false)
  (Variables|Default|SetCanPlaceRoad true))

(fn HideAll
  (for _array_element (Components|GetChildrenComponents (Variables|Default|GetDefaultSceneRoot) false)
    (bind _asmesh_component (Utilities|Casting|CastToMeshComponent _array_element))
    (Rendering|SetVisibility _asmesh_component false false)
    (Variables|Default|SetCanPlaceRoad false)
    (Variables|Default|SetCanDeleteRoad false)))

(fn ShowCross
  (CallFunction|HideAll)
  (Rendering|SetVisibility (Variables|Default|GetCross) true false)
  (Variables|Default|SetCanDeleteRoad true))