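; Road manager that lets the player place and remove road tiles on BP_Grid and lays the level's hard-coded starting roads.
; On BeginPlay it spawns a cursor road and grants starting roads through UI_PlayerInterface.
; While a build mode is active, Tick snaps the cursor to the grid under the mouse, previewing a road or removal cross by tile state.
; Placement spends a road, refunded on failure, and removal returns one.
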(event Custom|PlaceRoad
  (bind _cursorroad (Variables|Default|GetCursorRoad))
  (bind _returnvalue (Transformation|GetActorLocation _cursorroad))
  ;[1 1 1] Place Road
  (bind _haspaid (Default|PayRoad (Variables|Default|GetUIPlayerInterface)))
  (if _haspaid
    (if (Variables|/Game/Actor/Road/BP_RoadCursor.BP_RoadCursor_C|GetCanPlaceRoad _cursorroad)
      (bind _gridposition (Default|GetNearestGridCell (Variables|Default|GetGrid) (Math|Vector|MakeVector (.x _returnvalue) (.y _returnvalue) 0.0)))
      (bind _tileplaced (Default|PlaceRoadTile (Variables|Default|GetGrid) _gridposition))
      (if (not _tileplaced)
        (Default|GainRoad (Variables|Default|GetUIPlayerInterface) :!label _label))
      (else
        (goto _label)))))

(event Custom|RemoveRoad
  (bind _cursorroad (Variables|Default|GetCursorRoad))
  (bind _returnvalue (Transformation|GetActorLocation _cursorroad))
  ;[1 1 1] Remove Road
  (if (Variables|/Game/Actor/Road/BP_RoadCursor.BP_RoadCursor_C|GetCanDeleteRoad _cursorroad)
    (bind _gridposition (Default|GetNearestGridCell (Variables|Default|GetGrid) (Math|Vector|MakeVector (.x _returnvalue) (.y _returnvalue) 0.0)))
    (Default|RemoveRoadTile (Variables|Default|GetGrid) _gridposition)
    (Default|GainRoad (Variables|Default|GetUIPlayerInterface))))

(event EventBeginPlay
  ;[1 1 1] Initialise Cursor Road
  (bind _returnvalue (Game|SpawnActorfromClass "/Game/Actor/Road/BP_RoadCursor.BP_RoadCursor_C" (Math|Transform|MakeTransform "0.000000,0.000000,-1000.000000" "0, 0, 0" "1.000000,1.000000,1.000000") "Undefined" "MultiplyWithRoot" 0 0))
  (Variables|Default|SetCursorRoad _returnvalue)
  ;[1 1 1] init grid
  (bind _returnvalue_2 (Actor|GetActorOfClass "/Game/Blueprint/BP_Grid.BP_Grid_C"))
  (Variables|Default|SetGrid _returnvalue_2)
  (Utilities|FlowControl|Delay 0.2)
  ;[1 1 1] init player interface (for money)
  (bind _foundwidgets (Widget|GetAllWidgetsOfClass "/Game/UI/UI_PlayerInterface.UI_PlayerInterface_C" true))
  (bind _output_get (Variables|Default|SetUIPlayerInterface (Utilities|Array|Get(acopy) _foundwidgets)))
  (for _index (range 1 (Variables|Default|GetRoadStartAmount))
    (Default|GainRoad _output_get))
  (CallFunction|InitLevel))

(event EventTick
  (params (DeltaSeconds :type Float%20%28single-precision%29))
  (bind _grid (Variables|Default|GetGrid))
  (bind _cursorroad (Variables|Default|GetCursorRoad))
  (bind _returnvalue (Transformation|GetActorLocation _cursorroad))
  ;[1 1 1] Move CursorRoad
  (if (not (== (Variables|Default|GetBuildMode) ""))
    (CallFunction|MoveCursorRoad)
    (bind _gridposition (Default|GetNearestGridCell _grid (Math|Vector|MakeVector (.x _returnvalue) (.y _returnvalue) 0.0)))
    (bind _result (Default|GridPositionIsinGrid _grid _gridposition))
    (if _result
      (bind _isgridtilefree (Default|IsTileFree _grid _gridposition))
      (if _isgridtilefree
        (if (== (Variables|Default|GetBuildMode) "Place")
          (Default|ShowRoad (Variables|Default|GetCursorRoad))
          (else
            (Default|HideAll (Variables|Default|GetCursorRoad) :!label _label)))
        (else
          (bind _isroadtile (Default|IsTileRoad (Variables|Default|GetGrid) _gridposition))
          (if _isroadtile
            (if (== (Variables|Default|GetBuildMode) "Remove")
              (Default|ShowCross (Variables|Default|GetCursorRoad))
              (else
                (goto _label)))
            (else
              (goto _label)))))
      (else
        (goto _label)))))

(fn ConstructionScript)

(fn MoveCursorRoad
  (bind _returnvalue (Game|GetPlayerController 0))
  (bind _hitresult (Game|Player|GetHitResultUnderCursorbyChannel _returnvalue "TraceTypeQuery1" true))
  (bind _returnvalue_2 (+ (.y (.impactpoint _hitresult)) 1e+02))
  (bind _returnvalue_3 (+ (.x (.impactpoint _hitresult)) 1e+02))
  (if (!= (Variables|Default|GetBuildMode) "")
    (Transformation|SetActorLocation (Variables|Default|GetCursorRoad) (Math|Vector|MakeVector (- _returnvalue_3 (Math|Float|%(Float) _returnvalue_3 2e+02)) (- _returnvalue_2 (Math|Float|%(Float) _returnvalue_2 2e+02)) 0.0) false false)
    (else
      (Transformation|SetActorLocation (Variables|Default|GetCursorRoad) "0.000000,0.000000,-1000.000000" false false))))

(fn InitLevel
  ;[1 1 1] Spawn Roads
  (for _array_element (Utilities|Array|MakeArray "(X=7.000000,Y=0.000000)" "(X=7.000000,Y=1.000000)" "(X=7.000000,Y=2.000000)" "(X=7.000000,Y=3.000000)" "(X=7.000000,Y=4.000000)" "(X=5.000000,Y=5.000000)" "(X=4.000000,Y=5.000000)" "(X=4.000000,Y=6.000000)" "(X=4.000000,Y=7.000000)" "(X=5.000000,Y=7.000000)" "(X=6.000000,Y=7.000000)" "(X=9.000000,Y=7.000000)" "(X=9.000000,Y=8.000000)" "(X=9.000000,Y=9.000000)" "(X=8.000000,Y=9.000000)" "(X=7.000000,Y=9.000000)" "(X=7.000000,Y=10.000000)" "(X=7.000000,Y=11.000000)" "(X=7.000000,Y=12.000000)" "(X=7.000000,Y=13.000000)" "(X=7.000000,Y=14.000000)")
    (Default|PlaceRoadTile (Variables|Default|GetGrid) _array_element)))