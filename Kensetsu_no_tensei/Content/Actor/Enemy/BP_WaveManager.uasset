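; Wave manager that spawns ten scripted enemy waves for the defense phase and tracks their completion.
; SpawnWave switches on WaveNumber and runs delayed loops that count NumberToSpawn down through thresholds to mix enemy types, with boss music on the fifth and tenth waves.
; Spawn helpers raise EnemiesAlive at a fixed spawn point.
; DecreaseEnemy lowers that count and at zero advances the wave, then calls GainRoad on the player UI.
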(event Custom|SpawnWave
  (Audio|Components|Audio|SetSound (Variables|Default|GetAudioComponent) "/Game/Audios/AUDIO_DefensePhase.AUDIO_DefensePhase")
  (switch int (Variables|Default|GetWaveNumber)
    (:0
      ;[1 1 1] Waves 1 & 2
      (bind _output_get (Variables|Default|SetNumberToSpawn 5 :!label _label))
      (bind _isgreater (CallFunction|IsGreater _output_get :!label _label_2))
      (if _isgreater
        (CallFunction|SpawnBasicEnemy)
        (Utilities|FlowControl|Delay 2.0)
        (goto _label_2)))
    (:1
      (goto _label))
    (:2
      ;[1 1 1] Wave 3
      (bind _output_get_2 (Variables|Default|SetNumberToSpawn 10))
      (bind _isgreater_2 (CallFunction|IsGreater _output_get_2 4 :!label _label_3))
      (if _isgreater_2
        (CallFunction|SpawnBasicEnemy)
        (Utilities|FlowControl|Delay 2.0)
        (goto _label_3)
        (else
          (bind _isgreater_3 (CallFunction|IsGreater (Variables|Default|GetNumberToSpawn) :!label _label_4))
          (if _isgreater_3
            (CallFunction|SpawnFastEnemy)
            (Utilities|FlowControl|Delay 1.0)
            (goto _label_4)))))
    (:3
      ;[1 1 1] Wave 4
      (bind _output_get_3 (Variables|Default|SetNumberToSpawn 10))
      (bind _isgreater_4 (CallFunction|IsGreater _output_get_3 :!label _label_5))
      (if _isgreater_4
        (CallFunction|SpawnFastEnemy)
        (Utilities|FlowControl|Delay 1.0)
        (goto _label_5)))
    (:4
      ;[1 1 1] Wave 5
      (Audio|Components|Audio|SetSound (Variables|Default|GetAudioComponent) "/Game/Audios/AUDIO_BossPhase.AUDIO_BossPhase")
      (Variables|Default|SetNumberToSpawn 10)
      (CallFunction|SpawnSlowEnemy)
      (Utilities|FlowControl|Delay 2.0)
      (bind _isgreater_5 (CallFunction|IsGreater (Variables|Default|GetNumberToSpawn) 4 :!label _label_6))
      (if _isgreater_5
        (CallFunction|SpawnBasicEnemy)
        (Utilities|FlowControl|Delay 1.0)
        (goto _label_6)
        (else
          (bind _isgreater_6 (CallFunction|IsGreater (Variables|Default|GetNumberToSpawn) :!label _label_7))
          (if _isgreater_6
            (CallFunction|SpawnFastEnemy)
            (Utilities|FlowControl|Delay 1.0)
            (goto _label_7)))))
    (:5
      ;[1 1 1] Wave 6
      (bind _output_get_4 (Variables|Default|SetNumberToSpawn 5))
      (bind _isgreater_7 (CallFunction|IsGreater _output_get_4 :!label _label_8))
      (if _isgreater_7
        (CallFunction|SpawnRedBasicEnemy)
        (Utilities|FlowControl|Delay 1.0)
        (goto _label_8)))
    (:6
      ;[1 1 1] Wave 7
      (Variables|Default|SetNumberToSpawn 10)
      (CallFunction|SpawnSlowEnemy)
      (Utilities|FlowControl|Delay 1.0)
      (bind _isgreater_8 (CallFunction|IsGreater (Variables|Default|GetNumberToSpawn) 4 :!label _label_9))
      (if _isgreater_8
        (CallFunction|SpawnRedBasicEnemy)
        (Utilities|FlowControl|Delay 1.0)
        (goto _label_9)
        (else
          (bind _isgreater_9 (CallFunction|IsGreater (Variables|Default|GetNumberToSpawn) :!label _label_10))
          (if _isgreater_9
            (CallFunction|SpawnBasicEnemy)
            (Utilities|FlowControl|Delay 1.0)
            (goto _label_10)))))
    (:7
      ;[1 1 1] Wave 8
      (bind _output_get_5 (Variables|Default|SetNumberToSpawn 15))
      (bind _isgreater_10 (CallFunction|IsGreater _output_get_5 13 :!label _label_11))
      (if _isgreater_10
        (CallFunction|SpawnSlowEnemy)
        (Utilities|FlowControl|Delay 1.0)
        (goto _label_11)
        (else
          (bind _isgreater_11 (CallFunction|IsGreater (Variables|Default|GetNumberToSpawn) 8 :!label _label_12))
          (if _isgreater_11
            (CallFunction|SpawnRedBasicEnemy)
            (Utilities|FlowControl|Delay 1.0)
            (goto _label_12)
            (else
              (bind _isgreater_12 (CallFunction|IsGreater (Variables|Default|GetNumberToSpawn) 3 :!label _label_13))
              (if _isgreater_12
                (CallFunction|SpawnBasicEnemy)
                (Utilities|FlowControl|Delay 1.0)
                (goto _label_13)
                (else
                  (bind _isgreater_13 (CallFunction|IsGreater (Variables|Default|GetNumberToSpawn) 1 :!label _label_14))
                  (if _isgreater_13
                    (CallFunction|SpawnFastEnemy)
                    (Utilities|FlowControl|Delay 1.0)
                    (goto _label_14)
                    (else
                      (CallFunction|SpawnPurpleFastEnemy))))))))))
    (:8
      ;[1 1 1] Wave 9
      (bind _output_get_6 (Variables|Default|SetNumberToSpawn 20))
      (bind _isgreater_14 (CallFunction|IsGreater _output_get_6 17 :!label _label_15))
      (if _isgreater_14
        (CallFunction|SpawnFastEnemy)
        (Utilities|FlowControl|Delay 1.0)
        (goto _label_15)
        (else
          (bind _isgreater_15 (CallFunction|IsGreater (Variables|Default|GetNumberToSpawn) 15 :!label _label_16))
          (if _isgreater_15
            (CallFunction|SpawnSlowEnemy)
            (Utilities|FlowControl|Delay 1.0)
            (goto _label_16)
            (else
              (bind _isgreater_16 (CallFunction|IsGreater (Variables|Default|GetNumberToSpawn) 10 :!label _label_17))
              (if _isgreater_16
                (CallFunction|SpawnRedBasicEnemy)
                (Utilities|FlowControl|Delay 1.0)
                (goto _label_17)
                (else
                  (bind _isgreater_17 (CallFunction|IsGreater (Variables|Default|GetNumberToSpawn) 5 :!label _label_18))
                  (if _isgreater_17
                    (CallFunction|SpawnPurpleFastEnemy)
                    (Utilities|FlowControl|Delay 1.0)
                    (goto _label_18)
                    (else
                      (bind _isgreater_18 (CallFunction|IsGreater (Variables|Default|GetNumberToSpawn) :!label _label_19))
                      (if _isgreater_18
                        (CallFunction|SpawnBasicEnemy)
                        (Utilities|FlowControl|Delay 1.0)
                        (goto _label_19)))))))))))
    (:9
      ;[1 1 1] Wave 10
      (Audio|Components|Audio|SetSound (Variables|Default|GetAudioComponent) "/Game/Audios/AUDIO_BossPhase.AUDIO_BossPhase")
      (bind _output_get_7 (Variables|Default|SetNumberToSpawn 25))
      (bind _isgreater_19 (CallFunction|IsGreater _output_get_7 20 :!label _label_20))
      (if _isgreater_19
        (CallFunction|SpawnRedBasicEnemy)
        (Utilities|FlowControl|Delay 1.0)
        (goto _label_20)
        (else
          (bind _isgreater_20 (CallFunction|IsGreater (Variables|Default|GetNumberToSpawn) 15 :!label _label_21))
          (if _isgreater_20
            (CallFunction|SpawnBasicEnemy)
            (Utilities|FlowControl|Delay 1.0)
            (goto _label_21)
            (else
              (bind _isgreater_21 (CallFunction|IsGreater (Variables|Default|GetNumberToSpawn) 13 :!label _label_22))
              (if _isgreater_21
                (CallFunction|SpawnSlowEnemy)
                (Utilities|FlowControl|Delay 1.0)
                (goto _label_22)
                (else
                  (CallFunction|SpawnRedSlowEnemy)
                  (Utilities|FlowControl|Delay 1.0)
                  (bind _isgreater_22 (CallFunction|IsGreater (Variables|Default|GetNumberToSpawn) 10 :!label _label_23))
                  (if _isgreater_22
                    (CallFunction|SpawnSlowEnemy)
                    (Utilities|FlowControl|Delay 1.0)
                    (goto _label_23)
                    (else
                      (bind _isgreater_23 (CallFunction|IsGreater (Variables|Default|GetNumberToSpawn) 5 :!label _label_24))
                      (if _isgreater_23
                        (CallFunction|SpawnFastEnemy)
                        (Utilities|FlowControl|Delay 1.0)
                        (goto _label_24)
                        (else
                          (bind _isgreater_24 (CallFunction|IsGreater (Variables|Default|GetNumberToSpawn) :!label _label_25))
                          (if _isgreater_24
                            (CallFunction|SpawnPurpleFastEnemy)
                            (Utilities|FlowControl|Delay 1.0)
                            (goto _label_25)))))))))))))))

(event Custom|IncreaseWave
  (Math|Integer|IncrementInt (Variables|Default|GetWaveNumber)
    (:%20%20
      (Utilities|FlowControl|Delay 0.2)
      (Default|GainRoad (Variables|Default|GetUI_PlayerInterface)))))

(event Custom|DecreaseEnemy
  (bind _result (Math|Integer|DecrementInt (Variables|Default|GetEnemiesAlive))
    (:%20%20
      (bind _output_get (Variables|Default|SetEnemiesAlive _result))
      (if (== _output_get 0)
        (CallFunction|IncreaseWave)))))

(event EventBeginPlay
  (Variables|Default|SetWaveNumber 0)
  (Utilities|FlowControl|Delay 0.2)
  (bind _foundwidgets (Widget|GetAllWidgetsOfClass "/Game/UI/UI_PlayerInterface.UI_PlayerInterface_C" true))
  (Variables|Default|SetUI_PlayerInterface (Utilities|Array|Get(acopy) _foundwidgets)))

(fn ConstructionScript)

(fn SpawnBasicEnemy
  (if (> (Variables|Default|GetNumberToSpawn) 0)
    (Game|SpawnActorfromClass "/Game/Actor/Enemy/BP_BasicEnemy.BP_BasicEnemy_C" (Math|Conversions|ToTransform(Vector) "0.000000,0.000000,1000.000000") "Undefined" "MultiplyWithRoot" 0 0)
    (Math|Integer|IncrementInt (Variables|Default|GetEnemiesAlive)
      (:%20%20
        (Math|Integer|DecrementInt (Variables|Default|GetNumberToSpawn))))))

(fn SpawnFastEnemy
  (if (> (Variables|Default|GetNumberToSpawn) 0)
    (Game|SpawnActorfromClass "/Game/Actor/Enemy/BP_FastEnemy.BP_FastEnemy_C" (Math|Conversions|ToTransform(Vector) "0.000000,0.000000,1000.000000") "Undefined" "MultiplyWithRoot" 0 0)
    (Math|Integer|IncrementInt (Variables|Default|GetEnemiesAlive)
      (:%20%20
        (Math|Integer|DecrementInt (Variables|Default|GetNumberToSpawn))))))

(fn SpawnSlowEnemy
  (if (> (Variables|Default|GetNumberToSpawn) 0)
    (Game|SpawnActorfromClass "/Game/Actor/Enemy/BP_SlowEnemy.BP_SlowEnemy_C" (Math|Conversions|ToTransform(Vector) "0.000000,0.000000,1000.000000") "Undefined" "MultiplyWithRoot" 0 0)
    (Math|Integer|IncrementInt (Variables|Default|GetEnemiesAlive)
      (:%20%20
        (Math|Integer|DecrementInt (Variables|Default|GetNumberToSpawn))))))

(fn IsGreater
  (params (NumberToSpawn :type Integer) (RemainingNumber :type Integer))
  (return (> NumberToSpawn RemainingNumber)))

(fn SpawnRedBasicEnemy
  (if (> (Variables|Default|GetNumberToSpawn) 0)
    (Game|SpawnActorfromClass "/Game/Actor/Enemy/BP_BasicEnemyRed.BP_BasicEnemyRed_C" (Math|Conversions|ToTransform(Vector) "0.000000,0.000000,1000.000000") "Undefined" "MultiplyWithRoot" 0 0)
    (Math|Integer|IncrementInt (Variables|Default|GetEnemiesAlive)
      (:%20%20
        (Math|Integer|DecrementInt (Variables|Default|GetNumberToSpawn))))))

(fn SpawnRedSlowEnemy
  (if (> (Variables|Default|GetNumberToSpawn) 0)
    (Game|SpawnActorfromClass "/Game/Actor/Enemy/BP_SlowEnemyRed.BP_SlowEnemyRed_C" (Math|Conversions|ToTransform(Vector) "0.000000,0.000000,1000.000000") "Undefined" "MultiplyWithRoot" 0 0)
    (Math|Integer|IncrementInt (Variables|Default|GetEnemiesAlive)
      (:%20%20
        (Math|Integer|DecrementInt (Variables|Default|GetNumberToSpawn))))))

(fn SpawnPurpleFastEnemy
  (if (> (Variables|Default|GetNumberToSpawn) 0)
    (Game|SpawnActorfromClass "/Game/Actor/Enemy/BP_FastEnemyViolet.BP_FastEnemyViolet_C" (Math|Conversions|ToTransform(Vector) "0.000000,0.000000,1000.000000") "Undefined" "MultiplyWithRoot" 0 0)
    (Math|Integer|IncrementInt (Variables|Default|GetEnemiesAlive)
      (:%20%20
        (Math|Integer|DecrementInt (Variables|Default|GetNumberToSpawn))))))