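; Enemy character Blueprint that tracks health and shows it on a health bar widget component.
; BeginPlay sets health to the maximum and caches the BP_HealthBar widget, whose progress bar Tick refreshes every frame with the health ratio.
; AnyDamage subtracts incoming damage and destroys the actor when health reaches zero or below.
; An unconnected, unfinished rotation stub with a camera-location TODO never runs.
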(event Game|Damage|EventAnyDamage
  (params (Damage :type Float%20%28single-precision%29) (DamageType :type Damage%20Type%20Object%20Reference) (InstigatedBy :type Controller%20Object%20Reference) (DamageCauser :type Actor%20Object%20Reference))
  (if (> (Variables|Default|GetHeath) 0.0)
    (bind _output_get (Variables|Default|SetHeath (- (Variables|Default|GetHeath) Damage)))
    (if (<= _output_get 0.0)
      (Actor|DestroyActor))))

(event EventBeginPlay
  (Variables|Default|SetHeath (Variables|Default|GetMaxHealth))
  (bind _asbp_health_bar (Utilities|Casting|CastToBP_HealthBar (UserInterface|GetUserWidgetObject (Variables|Default|GetHealthBar))))
  (Variables|Default|SetAs%20BP%20Health%20Bar _asbp_health_bar))

(event EventTick
  (params (DeltaSeconds :type Float%20%28single-precision%29))
  (Progress|SetPercent (Variables|/Game/Actor/Enemy/BP_HealthBar.BP_HealthBar_C|GetHealthBar (Variables|Default|GetAs%20BP%20Health%20Bar)) (/ (Variables|Default|GetHeath) (Variables|Default|GetMaxHealth))))

(fn ConstructionScript)