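; BP_bullet is a tower projectile actor that damages whatever it hits.
; On BeginPlay it creates a dynamic material instance of MAT_Bullet on its Sphere and tints it with its Color variable.
; On Hit it applies Damage to the other actor, with no check on what that is, then destroys itself.
; Tick is empty; a linear position target aimed at Target is left disconnected, so it never runs.
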(event EventBeginPlay
  (bind _returnvalue (Rendering|Material|CreateDynamicMaterialInstance (Variables|Default|GetSphere) 0 "/Game/Actor/Towers/Bullets/MAT_Bullet.MAT_Bullet" "None" :!class /Script/Engine.PrimitiveComponent))
  ;[1 1 1] set color
  (Rendering|Material|SetVectorParameterValue _returnvalue "color" (Math|Conversions|ToLinearColor(Color) (Variables|Default|Getcolor)) :!class /Script/Engine.MaterialInstanceDynamic))

(event Collision|EventHit
  (params (MyComp :type Primitive%20Component%20Object%20Reference) (Other :type Actor%20Object%20Reference) (OtherComp :type Primitive%20Component%20Object%20Reference) (bSelfMoved :type Boolean) (HitLocation :type Vector :default "0, 0, 0") (HitNormal :type Vector :default "0, 0, 0") (NormalImpulse :type Vector :default "0, 0, 0") (Hit :type Hit%20Result%20Structure%20%28by%20ref%29))
  ;[1 1 1] Damage enemy
  (Game|Damage|ApplyDamage Other (Variables|Default|GetDamage) 0 0)
  (Actor|DestroyActor))

(event EventTick
  (params (DeltaSeconds :type Float%20%28single-precision%29))
  ;[1 1 1] not sure it works ?
)

(fn ConstructionScript)