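; PC_Click is the click-input handler for building roads and for placing and selecting turrets.
; On BeginPlay it caches the road and turret managers, then routes Place input to whichever build mode is active, with roads taking priority.
; Remove only deletes roads, as its turret branch is empty.
; Select traces under the cursor for a turret and sets a new upgrade widget on its Upgrades component.
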(event Input|EnhancedActionEvents|EnhancedInputActionSelect
  (params (ActionValue :type Boolean) (ElapsedSeconds :type Float%20%28double-precision%29) (TriggeredSeconds :type Float%20%28double-precision%29) (InputAction :type Input%20Action%20Object%20Reference :default "/Game/Input/Actions/Select.Select"))
  ;[1 1 1] Select Turret
  (:Started
    (bind _asbp_turret (Utilities|Casting|CastToBP_Turret (.hitactor (.HitResult (Game|Player|GetHitResultUnderCursorbyChannel (Game|GetPlayerController 0) "TraceTypeQuery1" true)))))
    (bind _returnvalue (UserInterface|CreateWidget "/Game/Actor/Towers/Upgrades/Ui_Upgrade.Ui_Upgrade_C" 0 _asbp_turret))
    (UserInterface|SetWidget (Variables|/Game/Actor/Towers/BP_Turret.BP_Turret_C|GetUpgrades _asbp_turret) _returnvalue)))

(event Input|EnhancedActionEvents|EnhancedInputActionPlace
  (params (ActionValue :type Boolean) (ElapsedSeconds :type Float%20%28double-precision%29) (TriggeredSeconds :type Float%20%28double-precision%29) (InputAction :type Input%20Action%20Object%20Reference :default "/Game/Input/Actions/Place.Place"))
  ;[1 1 1] Place Elements
  (:Started
    (if (== (Variables|/Game/Actor/Road/BP_RoadManager.BP_RoadManager_C|GetBuildMode (Variables|Default|GetRoad%20Manager)) "Place")
      (Default|PlaceRoad (Variables|Default|GetRoad%20Manager))
      (elif (!= (Variables|/Game/Actor/Towers/BP_TurretManager.BP_TurretManager_C|GetBuildMode (Variables|Default|GetTurret%20Manager)) "")
        (Default|PlaceTurret (Variables|Default|GetTurret%20Manager))))))

(event Input|EnhancedActionEvents|EnhancedInputActionRemove
  (params (ActionValue :type Boolean) (ElapsedSeconds :type Float%20%28double-precision%29) (TriggeredSeconds :type Float%20%28double-precision%29) (InputAction :type Input%20Action%20Object%20Reference :default "/Game/Input/Actions/Remove.Remove"))
  ;[1 1 1] Remove Elements
  (if (== (Variables|/Game/Actor/Road/BP_RoadManager.BP_RoadManager_C|GetBuildMode (Variables|Default|GetRoad%20Manager)) "Remove")
    (Default|RemoveRoad (Variables|Default|GetRoad%20Manager))
    (elif (!= (Variables|/Game/Actor/Towers/BP_TurretManager.BP_TurretManager_C|GetBuildMode (Variables|Default|GetTurret%20Manager)) "")
      _)))

(event EventBeginPlay
  ;[1 1 1] init
  (bind _returnvalue (Actor|GetActorOfClass "/Game/Actor/Road/BP_RoadManager.BP_RoadManager_C"))
  (Variables|Default|SetRoad%20Manager _returnvalue)
  (bind _returnvalue_2 (Actor|GetActorOfClass "/Game/Actor/Towers/BP_TurretManager.BP_TurretManager_C"))
  (Variables|Default|SetTurret%20Manager _returnvalue_2))

(fn ConstructionScript)