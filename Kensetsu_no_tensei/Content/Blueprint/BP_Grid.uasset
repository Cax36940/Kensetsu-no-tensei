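; Grid manager that builds a tile-based turret map on BeginPlay and tracks its occupancy.
; It fills every cell with a random small or hard clickable turret stored in the Terrain map, then spawns a straight middle-column road with actors beyond both ends.
; Helper functions convert between grid and world positions using origin and step, and add or remove entries in Roads and Towers maps keyed by cell.
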(event EventBeginPlay
  (bind _terrain (Variables|Default|GetTerrain))
  (Variables|Default|SetOriginPosition "")
  (Variables|Default|SetStep 2e+02)
  (bind _output_get (Variables|Default|SetGridSize "(X=15.000000,Y=15.000000)"))
  (for _index (range 1 (Math|Float|Truncate (.x _output_get)))
    (for _index_2 (range 1 (Math|Float|Truncate (.y _output_get)))
      (bind _position (CallFunction|GridPositiontoVector (Math|Vector2D|MakeVector2D (Math|Conversions|ToFloat(Integer) _index) (Math|Conversions|ToFloat(Integer) _index_2))))
      (if (Math|Random|RandomBool)
        (bind _returnvalue (Game|SpawnActorfromClass "/Game/Actor/Clickable/BP_ClickableSmallTurret.BP_ClickableSmallTurret_C" (Math|Conversions|ToTransform(Vector) _position) "Undefined" "MultiplyWithRoot" 0 0))
        (Utilities|Map|Add _terrain (Math|Vector2D|MakeVector2D (Math|Conversions|ToFloat(Integer) _index) (Math|Conversions|ToFloat(Integer) _index_2)) _returnvalue)
        (else
          (bind _returnvalue_2 (Game|SpawnActorfromClass "/Game/Actor/Clickable/BP_ClickableHardTurret.BP_ClickableHardTurret_C" (Math|Conversions|ToTransform(Vector) _position) "Undefined" "MultiplyWithRoot" 0 0))
          (Utilities|Map|Add _terrain (Math|Vector2D|MakeVector2D (Math|Conversions|ToFloat(Integer) _index) (Math|Conversions|ToFloat(Integer) _index_2)) _returnvalue_2)))))
  (bind _position_2 (CallFunction|GridPositiontoVector (Math|Vector2D|MakeVector2D (Math|Conversions|ToFloat(Integer) (Math|Float|Ceil (/ (.x (Variables|Default|GetGridSize)) 2.0))) 0.0)))
  (Game|SpawnActorfromClass "/Game/Actor/Road/BP_RoadEnd.BP_RoadEnd_C" (Math|Conversions|ToTransform(Vector) _position_2) "Undefined" "MultiplyWithRoot" 0 0)
  (bind _position_3 (CallFunction|GridPositiontoVector (Math|Vector2D|MakeVector2D (Math|Conversions|ToFloat(Integer) (Math|Float|Ceil (/ (.x (Variables|Default|GetGridSize)) 2.0))) (+ (.y (Variables|Default|GetGridSize)) 1.0))))
  (Game|SpawnActorfromClass "/Game/Actor/Road/BP_RoadEnd.BP_RoadEnd_C" (Math|Conversions|ToTransform(Vector) _position_3) "Undefined" "MultiplyWithRoot" 0 0)
  (for _index_3 (range 1 (Math|Float|Truncate (.y (Variables|Default|GetGridSize))))
    (bind _position_4 (CallFunction|GridPositiontoVector (Math|Vector2D|MakeVector2D (Math|Conversions|ToFloat(Integer) (Math|Float|Ceil (/ (.x (Variables|Default|GetGridSize)) 2.0))) (Math|Conversions|ToFloat(Integer) _index_3))))
    (Game|SpawnActorfromClass "/Game/Actor/Road/BP_RoadTile.BP_RoadTile_C" (Math|Conversions|ToTransform(Vector) _position_4) "Undefined" "MultiplyWithRoot" 0 0)))

(event Collision|EventActorBeginOverlap
  (params (OtherActor :type Actor%20Object%20Reference)))

(event EventTick
  (params (DeltaSeconds :type Float%20%28single-precision%29)))

(fn ConstructionScript)

(fn GridPositiontoVector
  (params (Vector :type Vector%202D%20Structure))
  (bind _originposition (Variables|Default|GetOriginPosition))
  (bind _step (Variables|Default|GetStep))
  (return (Math|Vector|MakeVector (+ (.x _originposition) (* (- (.x Vector) 1.0) _step)) (+ (.y _originposition) (* (- (.y Vector) 1.0) _step)) 0.0)))

(fn PlaceRoadTile
  (params (GridPosition :type Vector%202D%20Structure) (Tile :type BP%20Road%20Tile%20Object%20Reference))
  (Utilities|Map|Add (Variables|Default|GetRoads) GridPosition Tile))

(fn RemoveRoadTile
  (params (GridPosition :type Vector%202D%20Structure))
  (Utilities|Map|Remove (Variables|Default|GetRoads) GridPosition))

(fn GetNearestGridCell
  (params (VectorPosition :type Vector))
  (bind _step (Variables|Default|GetStep))
  (bind _originposition (Variables|Default|GetOriginPosition))
  (bind _step_2 (Variables|Default|GetStep))
  (bind _returnvalue (/ _step 2.0))
  (return (Math|Vector2D|MakeVector2D (Math|Conversions|ToFloat(Integer) (.ReturnValue (Math|Float|Division(WholeandRemainder) (- (+ (.x VectorPosition) _returnvalue) (.x _originposition)) _step_2))) (Math|Conversions|ToFloat(Integer) (.ReturnValue (Math|Float|Division(WholeandRemainder) (- (+ (.y VectorPosition) _returnvalue) (.y _originposition)) _step_2))))))

(fn PlaceTower
  (params (GridPosition :type Vector%202D%20Structure))
  (if (not (.ReturnValue (Utilities|Map|Find (Variables|Default|GetTowers) GridPosition)))
    (Utilities|Map|Add (Variables|Default|GetTowers) GridPosition true)))

(fn RemoveTower
  (params (GridPosition :type Vector%202D%20Structure))
  (Utilities|Map|Remove (Variables|Default|GetTowers) GridPosition))